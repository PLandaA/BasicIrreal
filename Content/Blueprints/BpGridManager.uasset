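; Wave manager that spawns zombie waves from BeginPlay and prints a win message once the last wave is cleared.
; Each wave totals four enemies per wave number, split between BP_Zombie and BP_Zombie2 at random locations within Utilities limits, passed through ValidCoord.
; EnemyKilled counts EnemyTotal down to zero, then WaveIncrement starts the next wave or ends at MaxWaves.
; EnemiesLeft is set at spawn but not decremented here.
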(event Custom|StartGame
  ;[1 1 1] StartGame
  (CallFunction|SpawnEnemies))

(event Custom|EnemyKilled
  ;[1 1 1] EnemyKilled
  (bind _result (Math|Integer|DecrementInt (Variables|Default|GetEnemyTotal))
    (:%20%20
      (if (== _result 0)
        (CallFunction|WaveIncrement)))))

(event Custom|SpawnEnemies
  (bind _utilities (Variables|Default|Getutilities))
  (bind _returnvalue (Class|UtilitiesInstance|MinLimits _utilities))
  (bind _returnvalue_2 (Class|UtilitiesInstance|MaxLimits _utilities))
  (bind _returnvalue_3 (Math|Random|RandomFloatinRange (.y _returnvalue) (.y _returnvalue_2)))
  (bind _returnvalue_4 (Math|Random|RandomFloatinRange (.x _returnvalue) (.x _returnvalue_2)))
  (bind _returnvalue_5 (Math|Vector|MakeVector _returnvalue_4 _returnvalue_3 5e+02))
  (bind _returnvalue_6 (Class|UtilitiesInstance|ValidCoord _utilities _returnvalue_5))
  (bind _returnvalue_7 (Math|Transform|MakeTransform _returnvalue_6))
  ;[1 1 1] SpawnEnemies
  (bind _output_get (Variables|Default|SetEnemyTotal (* (Variables|Default|GetCurrentWave) 4)))
  (Variables|Default|SetEnemiesLeft _output_get)
  (bind _index (Utilities|FlowControl|ForLoopwithBreak 0 _output_get :!label _label)
    (:LoopBody
      (if (== _index (/ (Variables|Default|GetEnemyTotal) 2))
        (goto _label Break)
        (else
          (bind _output_get_2 (Variables|Default|SetSpawnLocation1 _returnvalue_7))
          (Game|SpawnActorfromClass "/Game/Assets/Zombie/BP_Zombie.BP_Zombie_C" _output_get_2 "Undefined" "MultiplyWithRoot" 0 0))))
    (:Completed
      (Utilities|FlowControl|ForLoopwithBreak 1 (/ (Variables|Default|GetEnemyTotal) 2)
        (:LoopBody
          (bind _output_get_3 (Variables|Default|SetSpawnLocation2 _returnvalue_7))
          (Game|SpawnActorfromClass "/Game/Assets/Zombie/BP_Zombie2.BP_Zombie2_C" _output_get_3 "Undefined" "MultiplyWithRoot" 0 0))))))

(event Custom|WaveIncrement
  ;[1 1 1] WaveIncrement
  (if (== (Variables|Default|GetCurrentWave) (Variables|Default|GetMaxWaves))
    (Development|PrintString "Wins!")
    (else
      (Math|Integer|IncrementInt (Variables|Default|GetCurrentWave)
        (:%20%20
          (CallFunction|SpawnEnemies)
          (Development|PrintString "NextWave"))))))

(event EventBeginPlay
  ;[1 1 1] StartGame
  (CallFunction|StartGame))

(fn ConstructionScript)