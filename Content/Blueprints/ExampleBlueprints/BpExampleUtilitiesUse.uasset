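; Example actor that demonstrates the UtilitiesInstance API by printing the results of its queries on screen.
; Every Tick it casts the game instance to UtilitiesInstance, caches it in Utilities, then runs a sequence of sample calls.
; These cover asset paths, damage color and type conversions, obstacle and damage lookups by coordinate or transform, and min/max limits.
; Unconnected setup snippets and unused call nodes remain in both graphs, and the construction script does nothing.
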(event EventTick
  (params (DeltaSeconds :type Float%20%28single-precision%29))
  ;[0.3617 0 1 1 30] Global Example
  (bind _asutilities_instance (Utilities|Casting|CastToUtilitiesInstance (Game|GetGameInstance)))
  (bind _output_get (Variables|Default|SetUtilities _asutilities_instance))
  (Utilities|FlowControl|Sequence
    (:then_0
      (Development|PrintString (Class|UtilitiesInstance|AssetPath _output_get "FLOOR") true true "(R=1.000000,G=0.965018,B=0.000000,A=1.000000)" 6e+01))
    (:then_1
      (Development|PrintString (Utilities|String|ToString(Name) (Class|UtilitiesInstance|DamageColorName (Variables|Default|GetUtilities))) true true "(R=0.000000,G=0.660000,B=1.000000,A=1.000000)" 6e+01))
    (:then_2
      (Development|PrintString (Utilities|String|ToString(Boolean) (Class|UtilitiesInstance|ObstaclebyCoord (Variables|Default|GetUtilities) "246.000000,109.000000,0.000000"))))
    (:then_3
      (Development|PrintString "El tipo de color es el color de este texto" true true (Class|UtilitiesInstance|DamageColorbyType (Variables|Default|GetUtilities) (Utilities|Enum|LiteralenumDamageColor "GREEN")) 6e+01))
    (:then_4
      (Development|PrintString (Utilities|String|EnumtoString (Class|UtilitiesInstance|DamageTypebyColor (Variables|Default|GetUtilities) (Class|UtilitiesInstance|DamageColorbyType (Variables|Default|GetUtilities) (Utilities|Enum|LiteralenumDamageColor "GREEN")))) true true "(R=0.000000,G=0.660000,B=1.000000,A=1.000000)" 6e+01))
    (:then_5
      (Development|PrintString (Utilities|String|EnumtoString (Class|UtilitiesInstance|DamageTypebyTransform (Variables|Default|GetUtilities) (Transformation|GetActorTransform self))) true true "(R=0.000000,G=0.660000,B=1.000000,A=1.000000)" 6e+01))
    (:then_6
      (Development|PrintString (Utilities|String|ToString(Integer) (Class|UtilitiesInstance|MinLimits (Variables|Default|GetUtilities))) true true "(R=0.000000,G=1.000000,B=0.470675,A=1.000000)" 6e+01)
      (Development|PrintString "Min"))
    (:then_7
      (Development|PrintString (Utilities|String|ToString(Integer) (Class|UtilitiesInstance|MaxLimits (Variables|Default|GetUtilities))) true true "(R=0.000000,G=1.000000,B=0.473531,A=1.000000)" 6e+01)
      (Development|PrintString "Max"))
    (:then_8
      (Development|PrintString (Utilities|String|ToString(Vector) "-456.000000,1674.000000,0.000000") true true "(R=0.947642,G=1.000000,B=0.007734,A=1.000000)" 6e+01)
      (Development|PrintString (Utilities|String|EnumtoString (Class|UtilitiesInstance|DamageTypebyCoord (Variables|Default|GetUtilities) "-456.000000,1674.000000,0.000000")) true true "(R=1.000000,G=0.928552,B=0.000000,A=1.000000)" 6e+01))))

(fn ConstructionScript)